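; BP_CannonBall is a cannonball projectile that explodes on hit and damages nearby pawns.
; On Hit it spawns an explosion emitter at the impact point, hides its mesh and runs a sphere overlap for Pawns, ignoring itself.
; Each pawn found takes fixed damage with the ball as damage causer.
; The actor destroys itself only when the overlap finds a pawn; otherwise it remains with its mesh hidden.
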(event Collision|EventHit
  (params (MyComp :type Primitive%20Component%20Object%20Reference) (Other :type Actor%20Object%20Reference) (OtherComp :type Primitive%20Component%20Object%20Reference) (bSelfMoved :type Boolean) (HitLocation :type Vector :default "0, 0, 0") (HitNormal :type Vector :default "0, 0, 0") (NormalImpulse :type Vector :default "0, 0, 0") (Hit :type Hit%20Result%20Structure%20%28by%20ref%29))
  (Effects|SpawnEmitteratLocation "/Game/StarterContent/Particles/P_Explosion.P_Explosion" HitLocation)
  (Rendering|SetVisibility (Variables|Default|GetStaticMesh) false false)
  (bind (_outactors _returnvalue) (Collision|SphereOverlapActors HitLocation 5e+01 (Utilities|Array|MakeArray "ObjectTypeQuery3") 0 (Utilities|Array|MakeArray self)))
  (if _returnvalue
    (for _array_element _outactors
      (Game|Damage|ApplyDamage _array_element 1e+02 0 self "/Script/Engine.DamageType"))
    (Actor|DestroyActor)))

(fn ConstructionScript)