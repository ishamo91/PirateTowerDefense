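; BP_Cannon is a cannon item that turns to face humans it spots; it contains no firing logic.
; PawnSensing locks onto the first seen pawn tagged "Human" and starts a looping timer.
; The timer rotates the actor toward the target using interpolated look-at yaw.
; The lock persists regardless of sight until the target becomes invalid, which clears the timer and allows reacquisition.
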(event OnSeePawn(PawnSensing)
  (params (Pawn :type Pawn%20Object%20Reference))
  ;[0.15 0.15 0.15 0.5] Event see target
  (if (Actor|ActorHasTag Pawn "Human")
    (Utilities|IsValid Pawn
      (:Is%20Valid
        (if (not (Variables|Default|GetHasTarget?))
          (Variables|Default|SetHasTarget? true)
          (Variables|Default|SetTargetPawn Pawn)
          (CallFunction|TrackTarget))))))

(event Custom|TrackTarget
  ;[0.15 0.15 0.15 0.5] Rotate cannon to face target
  (bind _returnvalue (Utilities|Time|SetTimerbyEvent (delegate Custom|MoveCannon) 0.05 true true))
  (Variables|Default|SetTimerRef _returnvalue))

(event Custom|MoveCannon
  (bind _targetpawn (Variables|Default|GetTargetPawn))
  ;[0.15 0.15 0.15 0.5] Rotate cannon to face target
  (Utilities|IsValid _targetpawn
    (:Is%20Valid
      (Transformation|SetActorRotation (Math|Rotator|MakeRotator 0.0 0.0 (.yaw (Math|Interpolation|RInterpTo (Transformation|GetActorRotation) (Math|Rotator|FindLookatRotation (Transformation|GetActorLocation) (Transformation|GetActorLocation _targetpawn)) (Utilities|Time|GetWorldDeltaSeconds) 1e+02)))))
    (:Is%20Not%20Valid
      (Utilities|Time|ClearandInvalidateTimerbyHandle (Variables|Default|GetTimerRef))
      (Variables|Default|SetHasTarget? false))))

(fn ConstructionScript)