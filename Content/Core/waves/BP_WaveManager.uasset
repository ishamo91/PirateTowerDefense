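; Wave manager actor that spawns escalating waves of skeleton enemies.
; SpawnWave spawns the current quota of BP_Skeleton at the manager's location and counts them as alive.
; SkeletonDied decrements that count, then tests it minus one again, so the next, larger wave is scheduled after a delay while one skeleton is still counted alive.
; The first SpawnWave call is not made in this Blueprint.
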(event Custom|SpawnWave
  ;[0.15 0.15 0.15 0.5] Spawn Waves
  (Variables|Default|SetSkeletonsAlive 0)
  (for _index (range 1 (Variables|Default|GetSkeletonsToSpawn))
    (Game|SpawnActorfromClass "/Game/pirategameassets/animations/skeleton/BP_Skeleton.BP_Skeleton_C" (Math|Transform|MakeTransform (Transformation|GetActorLocation) "0, 0, 0" "1.000000,1.000000,1.000000") "Undefined" "MultiplyWithRoot" 0 0)
    (Variables|Default|SetSkeletonsAlive (+ (Variables|Default|GetSkeletonsAlive) 1))))

(event Custom|SkeletonDied
  ;[0.15 0.15 0.15 0.5] Next Wave
  (Variables|Default|SetSkeletonsAlive (- (Variables|Default|GetSkeletonsAlive) 1))
  (if (<= (- (Variables|Default|GetSkeletonsAlive) 1) 0)
    (Utilities|FlowControl|Delay 1e+01)
    (Variables|Default|SetSkeletonsToSpawn (+ (Variables|Default|GetSkeletonsToSpawn) 3))
    (CallFunction|SpawnWave)))

(fn ConstructionScript)