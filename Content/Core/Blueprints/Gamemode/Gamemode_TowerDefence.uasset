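; Tower defence game mode that runs skeleton waves and tracks the player's progress toward winning.
; On BeginPlay it caches spawn points, spawns the first wave at random points, then caches the first-person character.
; Skeleton count scales with wave number; reported kills count down until a short timer starts the next wave, or a win is printed after the last.
; Skeleton and wave counts are pushed to the character's UI.
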(event Custom|SpawnSkeletons
  (bind _characterref (Variables|Default|GetCharacterRef))
  ;[0.15 0.15 0.15 0.5] spawn skeles in game
  (bind _output_get (Variables|Default|SetSkeletonTotal (* (Variables|Default|GetCurrentWave) 4)))
  (Variables|Default|SetSkeletonsLeft _output_get)
  (for _index (range 1 (Variables|Default|GetSkeletonTotal))
    (Game|SpawnActorfromClass "/Game/Core/Blueprints/Skeleton/BP_Skeleton.BP_Skeleton_C" (Math|Transform|MakeTransform (Transformation|GetActorLocation (.OutItem (Utilities|Array|Random (Variables|Default|GetSpawnPoints)))) "0, 0, 0" "1.000000,1.000000,1.000000") "Undefined" "MultiplyWithRoot" 0 0))
  (Utilities|IsValid _characterref
    (:Is%20Valid
      (Class|BPIPirateCharacter|UpdateSkeletonsUI(Message) _characterref (Variables|Default|GetSkeletonsLeft) (Variables|Default|GetSkeletonTotal)))))

(event Custom|WaveIncrement
  (bind _characterref (Variables|Default|GetCharacterRef))
  ;[0.15 0.15 0.15 0.5] Check if player won game
  (if (== (Variables|Default|GetCurrentWave) (Variables|Default|GetMaxWaves))
    (Development|PrintString "Game Won")
    (else
      (Math|Integer|IncrementInt (Variables|Default|GetCurrentWave)
        (:%20%20
          (CallFunction|PreRoundTimer)))))
  (Utilities|IsValid _characterref
    (:Is%20Valid
      (Default|UpdateWavesUI _characterref (Variables|Default|GetCurrentWave) (Variables|Default|GetMaxWaves)))))

(event Custom|PreRoundTimer
  (Utilities|Time|SetTimerbyEvent (delegate Custom|StartNextWave) 5.0))

(event Custom|StartNextWave
  (CallFunction|SpawnSkeletons))

(event EventBeginPlay
  ;[0.15 0.15 0.15 0.5] set ref
  (Utilities|FlowControl|Sequence
    (:then_0
      (bind _outactors (Actor|GetAllActorsOfClass "/Game/Core/Blueprints/Skeleton/BP_SpawnPoint.BP_SpawnPoint_C"))
      (Variables|Default|SetSpawnPoints _outactors)
      (CallFunction|SpawnSkeletons))
    (:then_1
      (bind _outactors_2 (Actor|GetAllActorsOfClass "/Game/FirstPerson/Blueprints/BP_FirstPersonCharacter.BP_FirstPersonCharacter_C"))
      (Variables|Default|SetCharacterRef (Utilities|Array|Get(acopy) _outactors_2)))))

(event EventSkeletonKilled
  (bind _characterref (Variables|Default|GetCharacterRef))
  ;[0.15 0.15 0.15 0.5] Count Skeletons Killed
  (bind _result (Math|Integer|DecrementInt (Variables|Default|GetSkeletonsLeft))
    (:%20%20
      (if (== _result 0)
        (Development|PrintString "All skeletons killed")
        (CallFunction|WaveIncrement))
      (Utilities|IsValid _characterref
        (:Is%20Valid
          (Class|BPIPirateCharacter|UpdateSkeletonsUI(Message) _characterref (Variables|Default|GetSkeletonsLeft) (Variables|Default|GetSkeletonTotal)))))))

(fn ConstructionScript)