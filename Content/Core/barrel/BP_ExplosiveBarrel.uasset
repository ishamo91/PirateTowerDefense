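; Explosive barrel actor that takes damage and blows up when its health runs out.
; Any damage lowers BarrelHealth; at zero or below it spawns a scaled-up explosion emitter and fires the PushSkeletonsAway impulse.
; It then applies very high, full-strength radial damage over a wide radius, ignoring itself, and destroys the actor.
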(event Game|Damage|EventAnyDamage
  (params (Damage :type Float%20%28single-precision%29) (DamageType :type Damage%20Type%20Object%20Reference) (InstigatedBy :type Controller%20Object%20Reference) (DamageCauser :type Actor%20Object%20Reference))
  (bind _self self)
  (bind _returnvalue (Transformation|GetActorLocation _self))
  ;[0.15 0.15 0.15 0.5] Barrel explosion
  (bind _output_get (Variables|Default|SetBarrelHealth (- (Variables|Default|GetBarrelHealth) Damage)))
  (if (<= _output_get 0.0)
    (Effects|SpawnEmitteratLocation "/Game/StarterContent/Particles/P_Explosion.P_Explosion" _returnvalue "0, 0, 0" "10.000000,10.000000,10.000000")
    (Class|RadialForceComponent|FireImpulse (Variables|Default|GetPush%20Skeletons%20Away))
    (Game|Damage|ApplyRadialDamage 1e+05 _returnvalue 1.2e+03 "/Script/Engine.DamageType" (Utilities|Array|MakeArray self) 0 0 true "ECC_Visibility")
    (Actor|DestroyActor)))

(fn ConstructionScript)