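; Main menu pawn that puts the menu UI on screen and relays quality setting changes to it.
; On BeginPlay it creates W_MainMenu for player 0, adds it to the viewport, switches input to Game and UI and shows the mouse cursor.
; Its SetQualitySetting event forwards the setting and quality to the menu's options widget through SetQualitySettingMessage.
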(event EventBeginPlay
  (bind _returnvalue (Game|GetPlayerController 0))
  (Utilities|FlowControl|Sequence
    (:then_0
      (bind _returnvalue_2 (UserInterface|CreateWidget "/Game/Core/Widgets/MainMenu/W_MainMenu.W_MainMenu_C" (Game|GetPlayerController 0)))
      (bind _output_get (Variables|Default|SetMainMenuRef _returnvalue_2))
      (UserInterface|Viewport|AddtoViewport _output_get 0)
      (Input|SetInputModeGameandUI _returnvalue 0 "DoNotLock" true false)
      (Variables|/Script/Engine.PlayerController|SetbShowMouseCursor _returnvalue true))))

(event EventSetQualitySetting
  (params (Setting :type E_GraphicSetting%20Enum :default "NewEnumerator0") (Quality :type Integer))
  (Class|BPIMainMenuPawn|SetQualitySetting(Message) (Variables|/Game/Core/Widgets/MainMenu/W_MainMenu.W_MainMenu_C|GetOptionsWidget (Variables|Default|GetMainMenuRef)) Setting Quality))

(fn ConstructionScript)