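; Skeleton enemy character that marches at a random speed to a random point near the Keep and repeatedly attacks it.
; Pawn sensing gives a chance to chase and attack the player, gated by state flags that include already heading for the Keep.
; Both attacks apply sphere-overlap damage on montage notifies.
; Damage from non-Human causers updates the health bar; death triggers ragdoll, game mode notification and delayed destruction.
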(event OnSeePawn(PawnSensing)
  (params (Pawn :type Pawn%20Object%20Reference))
  ;[0.15 0.15 0.15 0.5] If see player, 30% chance to chase player
  (if (Actor|ActorHasTag Pawn "Player")
    (if (Math|Random|RandomBoolwithWeight 0.3)
      (if (not (Variables|Default|GetChasingPlayer?))
        (Variables|Default|SetPlayerRef Pawn)
        (CallFunction|ChasePlayer)))))

(event Custom|ChasePlayer
  ;[0.15 0.15 0.15 0.5] Attack Player Event
  (if (Math|Boolean|ANDBoolean (not (Variables|Default|GetIsDead?)) (not (Variables|Default|GetChasingPlayer?)) (not (Variables|Default|GetIsChasingKeep)) (not (Variables|Default|GetIsAttacking)))
    (Variables|Default|SetChasingPlayer? true)
    (AI|AIMoveTo self "0, 0, 0" (Variables|Default|GetPlayerRef) 5.0 false
      (:OnSuccess
        (CallFunction|AttackPlayer)))))

(event Custom|AttackPlayer
  ;[0.15 0.15 0.15 0.5] Attack Player
  (if (and (not (Variables|Default|GetIsDead?)) (not (Variables|Default|GetIsAttacking)))
    (Variables|Default|SetIsAttacking true)
    (Animation|Montage|PlayMontage (Variables|Character|GetMesh) "/Game/Core/Blueprints/Skeleton/Animations/A_Attack_Montage.A_Attack_Montage"
      (:OnCompleted
        (Variables|Default|SetIsAttacking false :!label _label)
        (Variables|Default|SetChasingPlayer? false)
        (CallFunction|ChasePlayer))
      (:OnInterrupted
        (goto _label))
      (:OnNotifyBegin
        (bind (_outactors _returnvalue) (Collision|SphereOverlapActors (Transformation|GetWorldLocation (Variables|Default|GetDamageRange)) 1e+02 (Utilities|Array|MakeArray "ObjectTypeQuery1" "ObjectTypeQuery2" "ObjectTypeQuery3") 0 (Utilities|Array|MakeArray self)))
        (if _returnvalue
          (for _array_element _outactors
            (Game|Damage|ApplyDamage _array_element 15.0 0 self "/Script/Engine.DamageType")))))))

(event Custom|SkeletonDeath
  (bind _charactermovement (Variables|Character|GetCharacterMovement))
  ;[0.15 0.15 0.15 0.5] Skeleton Death Logic
  (Variables|Default|SetIsDead? true)
  (Physics|SetSimulatePhysics (Variables|Character|GetMesh) true)
  (Collision|SetCollisionResponsetoChannel (Variables|Character|GetMesh) "ECC_Pawn" "ECR_Overlap")
  (Components|Movement|StopMovementImmediately _charactermovement)
  (Pawn|Components|CharacterMovement|DisableMovement _charactermovement)
  (Class|BPITowerDefenceGameMode|SkeletonKilled(Message) (Game|GetGameMode))
  (Utilities|FlowControl|Delay 1.25)
  (Actor|DestroyActor))

(event Custom|MoveToKeep
  ;[0.15 0.15 0.15 0.5] move to keep
  (if (Math|Boolean|ANDBoolean (not (Variables|Default|GetIsDead?)) (not (Variables|Default|GetIsChasingKeep)) (not (Variables|Default|GetChasingPlayer?)) (not (Variables|Default|GetIsAttacking)))
    (Variables|Default|SetIsChasingKeep true)
    (AI|AIMoveTo self (.RandomLocation (AI|Navigation|GetRandomReachablePointinRadius (Transformation|GetActorLocation (Variables|Default|GetKeepRef)) 2e+02 0 0)) 0 3e+01 true
      (:OnSuccess
        (CallFunction|DamageKeep))
      (:OnFail
        (Utilities|FlowControl|Delay 3.0)
        (Variables|Default|SetIsChasingKeep false)
        (CallFunction|MovetoKeep)))))

(event Custom|DamageKeep
  ;[0.15 0.15 0.15 0.5] Attack the Keep
  (if (and (not (Variables|Default|GetIsDead?)) (not (Variables|Default|GetIsDamagingKeep)))
    (Variables|Default|SetIsDamagingKeep true)
    (Animation|Montage|PlayMontage (Variables|Character|GetMesh) "/Game/Core/Blueprints/Skeleton/Animations/A_Attack_Montage.A_Attack_Montage"
      (:OnCompleted
        (Utilities|FlowControl|Delay (Math|Random|RandomFloatinRange 1.0 2.0) :!label _label)
        (Variables|Default|SetIsDamagingKeep false)
        (CallFunction|DamageKeep))
      (:OnInterrupted
        (goto _label))
      (:OnNotifyBegin
        (bind (_outactors _returnvalue) (Collision|SphereOverlapActors (Transformation|GetWorldLocation (Variables|Default|GetDamageRange)) 1e+02 (Utilities|Array|MakeArray "ObjectTypeQuery1" "ObjectTypeQuery2" "ObjectTypeQuery3") 0 (Utilities|Array|MakeArray self)))
        (if _returnvalue
          (Effects|SpawnEmitteratLocation "/Game/StarterContent/Particles/P_Ambient_Dust.P_Ambient_Dust" (Transformation|GetWorldLocation (Variables|Default|GetDamageRange)))
          (for _array_element _outactors
            (Game|Damage|ApplyDamage _array_element 25.0 0 self "/Script/Engine.DamageType")))))))

(event Collision|EventActorBeginOverlap
  (params (OtherActor :type Actor%20Object%20Reference)))

(event EventTick
  (params (DeltaSeconds :type Float%20%28single-precision%29)))

(event Game|Damage|EventAnyDamage
  (params (Damage :type Float%20%28single-precision%29) (DamageType :type Damage%20Type%20Object%20Reference) (InstigatedBy :type Controller%20Object%20Reference) (DamageCauser :type Actor%20Object%20Reference))
  ;[0.15 0.15 0.15 0.5] Skeleton damage
  (if (not (Actor|ActorHasTag DamageCauser "Human"))
    (if (not (Variables|Default|GetIsDead?))
      (if (<= (- (Variables|Default|GetHealth) Damage) 0.0)
        (Variables|Default|SetHealth (- (Variables|Default|GetHealth) Damage))
        (Class|BPISkeleHealthInterface|HideHealthBar(Message) (UserInterface|GetUserWidgetObject (Variables|Default|GetW_HealthBar)))
        (CallFunction|SkeletonDeath)
        (else
          (bind _output_get (Variables|Default|SetHealth (- (Variables|Default|GetHealth) Damage)))
          (Class|BPISkeleHealthInterface|UpdateHealth(Message) (UserInterface|GetUserWidgetObject (Variables|Default|GetW_HealthBar)) _output_get))))))

(event EventBeginPlay
  ;[0.15 0.15 0.15 0.5] Keep ref and move to it at random speed
  (bind _outactors (Actor|GetAllActorsOfClass "/Game/Core/Blueprints/Keep/BP_Keep.BP_Keep_C"))
  (for _array_element _outactors
    (Variables|Default|SetKeepRef _array_element))
  (CallFunction|MovetoKeep)
  (Variables|/Script/Engine.CharacterMovementComponent|SetMaxWalkSpeed (Variables|Character|GetCharacterMovement) (Math|Random|RandomFloatinRange 3e+02 4e+02)))

(fn ConstructionScript)