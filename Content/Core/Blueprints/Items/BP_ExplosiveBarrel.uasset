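; BP_ExplosiveBarrel is a destructible barrel that explodes the first time it takes any damage.
; A DoOnce gate spawns an enlarged explosion particle effect, then sphere-overlaps nearby Pawns, applies flat damage to each, and destroys the barrel.
; Because the overlap only queries Pawn object types, the blast has no falloff and only chain-reacts with other barrels if they use that object type.
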(event Game|Damage|EventAnyDamage
  (params (Damage :type Float%20%28single-precision%29) (DamageType :type Damage%20Type%20Object%20Reference) (InstigatedBy :type Controller%20Object%20Reference) (DamageCauser :type Actor%20Object%20Reference))
  (Utilities|FlowControl|DoOnce false
    (:Completed
      (Effects|SpawnEmitteratLocation "/Game/StarterContent/Particles/P_Explosion.P_Explosion" (Transformation|GetActorLocation) "0, 0, 0" "6.000000,6.000000,6.000000")
      (bind (_outactors _returnvalue) (Collision|SphereOverlapActors (Transformation|GetActorLocation) 3e+02 (Utilities|Array|MakeArray "ObjectTypeQuery3") 0 (Utilities|Array|MakeArray self)))
      (if _returnvalue
        (for _array_element _outactors
          (Game|Damage|ApplyDamage _array_element 1e+02 0 self "/Script/Engine.DamageType")))
      (Actor|DestroyActor))))

(fn ConstructionScript)